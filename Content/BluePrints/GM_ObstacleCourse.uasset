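; Game mode for the obstacle course level that sets up level state, UI and a repeating timer.
; BeginPlay sets game-only input, creates but does not display an end screen, and adds the HUD to the viewport.
; It records the current level in the multi-level game instance and sets the win screen as next.
; A looping timer increments the game instance's counter and refreshes the HUD's timer text.
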(event Custom|IncrementCount
  (Default|IncrementCounter (Variables|Default|GetGIRef))
  (Default|SetTimerText (Variables|Default|GetUIRef)))

(event EventBeginPlay
  (Input|SetInputModeGameOnly (Game|GetPlayerController 0) false)
  (bind _returnvalue (UserInterface|CreateWidget "/Game/UI/EndScreen.EndScreen_C"))
  (Variables|Default|SetEndScreenRef _returnvalue)
  (bind _asgi_multi_level (Utilities|Casting|CastToGI_MultiLevel (Game|GetGameInstance)))
  (bind _output_get (Variables|Default|SetGIRef _asgi_multi_level))
  (Variables|/Game/BluePrints/GI_MultiLevel.GI_MultiLevel_C|SetIsPaused _output_get false)
  (bind _returnvalue_2 (Game|GetCurrentLevelName true))
  (Variables|/Game/BluePrints/GI_MultiLevel.GI_MultiLevel_C|SetCurrentLevelName _output_get _returnvalue_2)
  (Variables|/Game/BluePrints/GI_MultiLevel.GI_MultiLevel_C|SetNextLevelName _output_get "L_WinScreen")
  (Actor|GetAllActorsOfClass "/Game/ThirdPerson/Blueprints/BP_ThirdPersonCharacter.BP_ThirdPersonCharacter_C")
  (bind _returnvalue_3 (UserInterface|CreateWidget "/Game/UI/WBP_UI.WBP_UI_C"))
  (bind _output_get_2 (Variables|Default|SetUIRef _returnvalue_3))
  (UserInterface|Viewport|AddtoViewport _output_get_2 0)
  (Utilities|Time|SetTimerbyEvent (delegate Custom|IncrementCount) (Variables|Default|GetIncrementCounts) true))

(fn ConstructionScript)